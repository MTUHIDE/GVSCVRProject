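; RTS player controller that drives the camera pawn and handles object clicks and building placement.
; BeginPlay caches pawn and game state, spawns the construction manager and ghost building, and creates the main HUD.
; Key and screen-edge input pan the camera at zoom- or Shift-scaled speeds, alongside clamped zoom.
; In build mode the ghost follows the cursor and left-click queues construction; otherwise clicked objects go to a HUD request.
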(event EventBeginPlay
  (bind _returnvalue (Math|Transform|MakeTransform "0, 0, 0"))
  ;[1 1 1] Begin Play
  (Utilities|FlowControl|Sequence
    (:then_0
      (Utilities|ReferenceCasts))
    (:then_1
      (bind _returnvalue_2 (Game|SpawnActorfromClass "/Game/RTS/Blueprints/Construction/ConstructionManager_BP.ConstructionManager_BP_C" _returnvalue "AlwaysSpawn" 0 0))
      (Variables|References|SetConstructionManagerRef _returnvalue_2))
    (:then_2
      (bind _returnvalue_3 (Game|SpawnActorfromClass "/Game/RTS/Blueprints/Buildings/GhostBuilding_BP.GhostBuilding_BP_C" _returnvalue "AlwaysSpawn" 0 self 0))
      (Variables|References|SetGhostBuildingRef _returnvalue_3))
    (:then_3
      (Input|SetInputModeGameandUI self 0 "LockInFullscreen" true)
      (Utilities|CreateHuds)
      (UserInterface|Viewport|AddtoViewport (Variables|References|GetMainHudRef) 0))))

(event EventTick
  (params (DeltaSeconds :type Float%20%28single-precision%29))
  (Utilities|FlowControl|Sequence
    (:then_0
      ;[1 1 1] Follow Cursor during Build Mode
      (if (Variables|Default|GetBuildModeActive)
        (|SetCursorWorldPosition)))
    (:then_1
      (if (Class|HeadMountedDisplayFunctionLibrary|IsHeadMountedDisplayEnabled)
        (if (Class|HeadMountedDisplayFunctionLibrary|IsHeadMountedDisplayConnected)
          (Transformation|SetActorTransform self (CallFunction|VRRotationTransform)))))))

(event Input|ActionEvents|InputActionZoomIn
  (params (Key :type Key%20Structure :default "None"))
  (bind _camerapawnref (Variables|References|GetCameraPawnRef))
  (bind _springarm (Variables|/Game/RTS/Blueprints/CameraPawn.CameraPawn_C|GetSpringArm _camerapawnref))
  ;[1 1 1] Zoom In and Out
  (:Pressed
    (Variables|/Script/Engine.SpringArmComponent|SetTargetArmLength _springarm (Math|Float|Clamp(Float) (- (Variables|/Script/Engine.SpringArmComponent|GetTargetArmLength _springarm) (Variables|Default|GetZoomSensitivity)) 5e+02 (Variables|Default|GetMaxArmDistance)))))

(event Input|ActionEvents|InputActionZoomOut
  (params (Key :type Key%20Structure :default "None"))
  (bind _camerapawnref (Variables|References|GetCameraPawnRef))
  (bind _springarm (Variables|/Game/RTS/Blueprints/CameraPawn.CameraPawn_C|GetSpringArm _camerapawnref))
  ;[1 1 1] Zoom In and Out
  (:Pressed
    (Variables|/Script/Engine.SpringArmComponent|SetTargetArmLength _springarm (Math|Float|Clamp(Float) (+ (Variables|Default|GetZoomSensitivity) (Variables|/Script/Engine.SpringArmComponent|GetTargetArmLength _springarm)) 5e+02 (Variables|Default|GetMaxArmDistance)))))

(event Input|ActionEvents|InputActionZoomReset
  (params (Key :type Key%20Structure :default "None"))
  ;[1 1 1] Zoom Reset
  (:Pressed
    (Variables|/Script/Engine.SpringArmComponent|SetTargetArmLength (Variables|/Game/RTS/Blueprints/CameraPawn.CameraPawn_C|GetSpringArm (Variables|References|GetCameraPawnRef)) 1.5e+03)))

(event Input|ActionEvents|InputActionDeselect
  (params (Key :type Key%20Structure :default "None"))
  (:Pressed
    (if (Variables|Default|GetBuildModeActive)
      (Default|KillGhost (Variables|References|GetGhostBuildingRef))
      (Variables|Default|SetBuildModeActive false))))

(event Input|AxisEvents|InputAxisMoveForward
  (params (AxisValue :type Float%20%28single-precision%29))
  ;[1 1 1] Movement X
  (if (not (Variables|Default|GetDisableCamNav))
    (Transformation|SetActorTransform (Variables|References|GetCameraPawnRef) (Utilities|MovementX (CallFunction|MovementSpeedCalculation) (Variables|Default|GetFastMoveMultiplier) AxisValue (Variables|References|GetCameraPawnRef)))))

(event Input|AxisEvents|InputAxisMoveRight
  (params (AxisValue :type Float%20%28single-precision%29))
  (bind _movementsensitivity (CallFunction|MovementSpeedCalculation))
  (bind _fastmovemultiplier (Variables|Default|GetFastMoveMultiplier))
  (bind _camerapawnref (Variables|References|GetCameraPawnRef))
  (bind _transform (Utilities|MovementY AxisValue _movementsensitivity _fastmovemultiplier _camerapawnref))
  (bind (_location _rotation _scale) (Math|Transform|BreakTransform _transform))
  (bind (_x _y) (Math|Vector|BreakVector _location))
  ;[1 1 1] Movement Y
  (if (not (Variables|Default|GetDisableCamNav))
    (Transformation|SetActorTransform (Variables|References|GetCameraPawnRef) (Math|Transform|MakeTransform (Math|Vector|MakeVector _x _y 1e+02) _rotation _scale))))

(event Input|MouseEvents|MouseX
  (params (AxisValue :type Float%20%28single-precision%29))
  ;[1 1 1] ScreenEdge Movement
  (if (not (Variables|Default|GetDisableCamNav))
    (bind (_deltaxspeed _deltayspeed) (Utilities|ScreenEdgeMovement))
    (Transformation|AddActorLocalOffset (Variables|References|GetCameraPawnRef) (Math|Vector|MakeVector _deltaxspeed _deltayspeed 0.0) true false)))

(event Input|MouseEvents|MouseY
  (params (AxisValue :type Float%20%28single-precision%29))
  ;[1 1 1] ScreenEdge Movement
  (if (not (Variables|Default|GetDisableCamNav))
    (Utilities|ScreenEdgeMovement) ; enters at MouseY
  ))

(event Input|KeyboardEvents|V
  (params (Key :type Key%20Structure :default "None"))
  (bind _self self)
  (bind _location (CallFunction|SetCursorWorldPosition _self 1e+02))
  ;[1 1 1] Spawn NPC (Temp)
  (:Pressed
    (Game|SpawnActorfromClass "/Game/RTS/Blueprints/AI/NPC_Basic.NPC_Basic_C" (Math|Transform|MakeTransform (.location (Math|Transform|MakeTransform (Math|Vector|MakeVector (.x _location) (.y _location) 218.0))) "0, 0, 0" "1,1,1") "AlwaysSpawn" 0 0)))

(event Input|MouseEvents|LeftMouseButton
  (params (Key :type Key%20Structure :default "None"))
  (bind _selectableobjectsenum (Variables|Default|GetSelectableObjectsENUM))
  (bind _hitresult (Class|PlayerController|GetHitResultUnderCursorforObjects _selectableobjectsenum true))
  (bind _hitactor (Collision|BreakHitResult _hitresult))
  ;[1 1 1] Left Mouse Button
  (:Pressed
    (if (Variables|Default|GetBuildModeActive)
      (if (|VerifyAsPlaceable)
        (bind _constructionstruct (Default|GetConstructionStruct (Variables|References|GetGhostBuildingRef)))
        (Default|QueueConstruction (Variables|References|GetConstructionManagerRef) _constructionstruct)
        (Default|KillGhost (Variables|References|GetGhostBuildingRef)))
      (elif (!= _hitactor 0)
        (Default|CallHUDRequest _hitactor)))))

(event Input|KeyboardEvents|LeftShift
  (params (Key :type Key%20Structure :default "None"))
  ;[1 1 1] Movement Multiplyer
  (:Pressed
    (Variables|Default|SetFastMoveMultiplier 2.0))
  (:Released
    (Variables|Default|SetFastMoveMultiplier 1.0)))

(event Input|MouseEvents|RightMouseButton
  (params (Key :type Key%20Structure :default "None"))
  ;[1 1 1] Left Mouse Button
  (:Pressed
    (bind _output_get (Variables|Default|SetMoveRef (CallFunction|SetCursorWorldPosition self (CallFunction|SetSightDistance))))
    (Development|PrintString (Utilities|String|ToString(Vector) _output_get))))

(event Input|KeyboardEvents|LeftShift
  (params (Key :type Key%20Structure :default "None"))
  (:Pressed
    (Variables|Default|SetSelectMultiple true))
  (:Released
    (Variables|Default|SetSelectMultiple false)))

(fn ConstructionScript)

(fn MovementSpeedCalculation
  (return (Math|Float|Clamp(Float) (/ (Variables|/Script/Engine.SpringArmComponent|GetTargetArmLength (Variables|/Game/RTS/Blueprints/CameraPawn.CameraPawn_C|GetSpringArm (Variables|References|GetCameraPawnRef))) 1e+02) 5.0 2e+01)))

(fn SetSightDistance
  (return (+ (Variables|Default|GetSightDistance) (Variables|/Script/Engine.SpringArmComponent|GetTargetArmLength (Variables|/Game/RTS/Blueprints/CameraPawn.CameraPawn_C|GetSpringArm (Variables|References|GetCameraPawnRef))))))

(fn VRRotationTransform
  (bind _devicerotation (Class|HeadMountedDisplayFunctionLibrary|GetOrientationandPosition))
  (bind _self self)
  (bind _returnvalue (Transformation|GetActorTransform _self))
  (return (Math|Transform|MakeTransform (.location _returnvalue) (Math|Rotator|MakeRotator (.roll _devicerotation) (.pitch _devicerotation) (- (.yaw _devicerotation) 7e+01)) (.scale _returnvalue))))

(fn SetCalendar
  (params (Date :type Array%20of%20Integers))
  (return false))

(fn SetClock
  (params (Time :type Array%20of%20Integers))
  (return false))