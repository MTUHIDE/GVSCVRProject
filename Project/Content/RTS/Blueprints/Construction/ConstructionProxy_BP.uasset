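; Ghost-material placeholder building for the RTS that tracks construction time, then announces completion and destroys itself.
; Tick advances a clock scaled by the GameState's game-speed updates until the required construction time is reached.
; Workers register through ReportToShift and ConstructionComplete frees and unhides them, but their count does not affect build speed.
; A HUD request glides the camera to the proxy and opens its widget, locking camera navigation and the main HUD.
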(event Custom|AdjustTime
  (params (TimeUnit :type Float%20%28single-precision%29))
  (Variables|Default|SetTimeUnit TimeUnit))

(event Custom|DisplayHUD
  (params (Actor :type Actor%20Object%20Reference))
  (bind _controllerref (Variables|Default|GetControllerRef))
  ;[1 1 1] Display HUD
  (if (== Actor self)
    (Utilities|FlowControl|Sequence
      (:then_0
        (bind _newlocation (|LerpLocation)
          (:Update
            (Transformation|SetActorLocation (Variables|/Game/RTS/Blueprints/CameraPawnController.CameraPawnController_C|GetCameraPawnRef (Variables|Default|GetControllerRef)) _newlocation false false))))
      (:then_1
        (UserInterface|Viewport|AddtoViewport (Variables|Default|GetProxy_HUD) 0)
        (Input|SetInputModeUIOnly _controllerref 0 "LockOnCapture")
        (Variables|/Game/RTS/Blueprints/CameraPawnController.CameraPawnController_C|SetDisableCamNav _controllerref true)
        (Widget|SetIsEnabled (Variables|/Game/RTS/Blueprints/CameraPawnController.CameraPawnController_C|GetMainHudRef _controllerref) false)))))

(event EventBeginPlay
  (bind _output_get (Variables|Default|SetGameStateReference (.AsGame%20State (Utilities|Casting|CastToGameState (Game|GetGameState)))))
  (EventDispatchers|BindEventtoUpdateGameSpeed _output_get (EventDispatchers|CreateEvent :!event Custom|AdjustTime))
  (bind _ascamera_pawn_controller (Utilities|Casting|CastToCameraPawnController (Game|GetPlayerController 0)))
  (bind _output_get_2 (Variables|Default|SetControllerRef _ascamera_pawn_controller))
  (EventDispatchers|BindEventtoHUDRequest _output_get_2 (EventDispatchers|CreateEvent :!event Custom|DisplayHUD))
  (bind _returnvalue (UserInterface|CreateWidget "/Game/RTS/HUDs/Proxy_HUD.Proxy_HUD_C" 0 self (Variables|Default|GetControllerRef)))
  (Variables|Default|SetProxy_HUD _returnvalue))

(event EventTick
  (params (DeltaSeconds :type Float%20%28single-precision%29))
  (Variables|Default|SetDelta DeltaSeconds)
  (if (not (Variables|Default|GetisConstructedCompleted))
    (CallFunction|DoWork)
    (if (>= (Variables|Default|GetWorkTimeSpent) (Variables|Default|GetConstructionTime))
      (Variables|Default|SetisConstructedCompleted true)
      (Default|CallConstructionCompleted self)
      (if (UserInterface|Viewport|IsinViewport (Variables|Default|GetProxy_HUD))
        (Default|RemoveHUD (Variables|Default|GetProxy_HUD)))
      (Utilities|FlowControl|Delay 0.2)
      (Actor|DestroyActor))))

(fn ConstructionScript
  (bind _staticmesh (Variables|Default|GetStaticMesh))
  (Components|StaticMesh|SetStaticMesh _staticmesh (Variables|Default|GetDisplayMesh))
  (Rendering|Material|SetMaterial _staticmesh 0 "/Game/RTS/Materials/Ghost_M_Inst.Ghost_M_Inst")
  (CallFunction|SetBuildingEntrance (Variables|Default|GetEntrance) (Variables|Default|GetStaticMesh))
  (CallFunction|SetBuildingCollision (Variables|Default|GetCollision) (Variables|Default|GetStaticMesh)))

(fn SetConstructionTime
  (params (WorkHours :type Float%20%28single-precision%29))
  (Variables|Default|SetConstructionTime (* WorkHours 6e+01))
  (return))

(fn DoWork
  (bind _output_get (Variables|Default|SetClockwork (.ClockworkOut (CallFunction|SetClockwork (Variables|Default|GetDelta) (Variables|Default|GetTimeUnit) (Variables|Default|GetClockwork)))))
  (Variables|Default|SetWorkTimeSpent (* _output_get 6e+01))
  (return))

(fn GetWorkForce
  (return (Math|Conversions|ToFloat(Integer) (Utilities|Array|Length (Variables|Default|GetActiveWorkers)))))

(fn ReporttoShift
  (params (Worker :type NPC%20Basic%20Object%20Reference))
  (Utilities|Array|Add (Variables|Default|GetActiveWorkers) Worker)
  (return))

(fn ConstructionComplete
  (if (> (CallFunction|GetWorkForce) 0.0)
    (for _array_element (Variables|Default|GetActiveWorkers)
      (Default|SetIsBusy _array_element false)
      (Rendering|SetActorHiddenInGame _array_element false))
    (Variables|Default|SetActiveWorkers (Utilities|Array|MakeArray 0))
    (return)
    (else
      (return))))