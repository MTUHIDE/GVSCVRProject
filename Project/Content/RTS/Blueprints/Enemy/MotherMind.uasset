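; MotherMind is an RTS enemy brain that spawns units from a Base and switches between Attack and Defend strategies.
; A scaled countdown spawns units into a tracked collection, catching up on missed intervals.
; Strategy flips on thresholds combining unit count and time since the last switch, then calls EmployStrategy.
; The Tick logic is disconnected, and EmployStrategy's per-unit strategy switch is still empty.
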(event EventBeginPlay
  (Variables|Default|SetDelayCountdown (Variables|Default|GetSpawnDelay)))

(event EventTick
  (params (DeltaSeconds :type Float%20%28single-precision%29))
  ;[1 1 1] Connect to enable
)

(fn ConstructionScript)

(fn SpawnCountdown
  (params (DeltaTime :type Float%20%28single-precision%29))
  (bind _deltasecondsout (CallFunction|RealSecondstoDeltaSeconds DeltaTime self))
  (bind _output_get (Variables|Default|SetDelayCountdown (- (Variables|Default|GetDelayCountdown) _deltasecondsout)))
  (if (< _output_get 0.0) :!label _label
    (Variables|Default|SetDelayCountdown (+ (Variables|Default|GetSpawnDelay) (Variables|Default|GetDelayCountdown)))
    (bind _newparam (Default|SpawnUnit (Variables|Default|GetBase)))
    (Utilities|Set|Add (Variables|Default|GetUnits) _newparam)
    (goto _label)))

(fn ChooseStrategy
  ;[1 1 1] some calculation to determine what strategy to use
  (switch Utilities|FlowControl|Switch|SwitchonStrategies (Variables|Default|GetStrategy)
    (:NewEnumerator0
      (if (< (/ (Math|Float|Sqrt (Math|Conversions|ToFloat(Integer) (Utilities|Set|Length (Variables|Default|GetUnits)))) (Variables|Default|GetTimeSenceLastAttack)) 0.0001)
        (Variables|Default|SetTimeSenceLastAttack 0.0)
        (Variables|Default|SetStrategy "NewEnumerator1")
        (CallFunction|EmployStrategy (Variables|Default|GetUnits))))
    (:NewEnumerator1
      (if (> (* (Utilities|Set|Length (Variables|Default|GetUnits)) (Variables|Default|GetTimeSenceLastAttack)) 1e+05)
        (Variables|Default|SetTimeSenceLastAttack 0.0)
        (Variables|Default|SetStrategy "NewEnumerator0")
        (CallFunction|EmployStrategy (Variables|Default|GetUnits))))))

(fn EmployStrategy
  (params (Units :type Set%20of%20NPC%20Basic%20Object%20References))
  (bind _result (Utilities|Set|ToArray Units))
  (for _array_element _result
    (switch Utilities|FlowControl|Switch|SwitchonStrategies (Variables|Default|GetStrategy))))