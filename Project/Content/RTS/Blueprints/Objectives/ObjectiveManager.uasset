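; Objective manager for the RTS game that owns the list of objectives and their on-screen ObjectivesPanel widget.
; BeginPlay creates the panel, and Setup passes the manager and panel to each objective.
; TestForObjectivesCompletion opens a gate, closes it if any objective is incomplete, then enters it, so completion currently only prints a message when all are done.
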(event EventBeginPlay
  ;[1 1 1] Creates an Objectives Panel
  (bind _returnvalue (UserInterface|CreateWidget "/Game/RTS/HUDs/ObjectivesPanel.ObjectivesPanel_C" (Game|GetPlayerController 0)))
  (bind _output_get (Variables|Default|SetobjectivesPanel _returnvalue))
  (UserInterface|Viewport|AddtoViewport _output_get 0))

(fn ConstructionScript)

(fn TestforObjectivesCompletion
  ;[1 1 1] Tests if all objectives have been completed, and for now will print "All Objectives Completed" to the console
  (Utilities|FlowControl|Sequence
    (:then_0
      (goto _label Open))
    (:then_1
      (for _array_element (Variables|Default|Getobjectives)
        (if (not (Variables|/Game/RTS/Blueprints/Objectives/Objective.Objective_C|Getcomplete _array_element))
          (goto _label Close)))
      (if true
        (Utilities|FlowControl|Gate false :!label _label ; Exit only if all objective are completed
          (:Exit
            (Development|PrintString "All Objectives Completed")))))))

(fn Setup
  ;[1 1 1] Calls Setup for each Objective
  (for _array_element (Variables|Default|Getobjectives)
    (Default|Setup _array_element self (Variables|Default|GetobjectivesPanel))))