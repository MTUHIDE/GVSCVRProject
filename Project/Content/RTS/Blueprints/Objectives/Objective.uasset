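; Base objective for the RTS that tracks progress toward a target value and shows it as an entry in the objectives panel.
; Setup stores the objective manager and creates its panel entry with the task name and goal.
; SetCompletion, also reached through ChangeCompletion for increments, updates the entry, marks completion once the target is reached, and then has the manager test for objectives completion.
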(event EventTick
  (params (DeltaSeconds :type Float%20%28single-precision%29)))

(fn ConstructionScript)

(fn SetCompletion
  (params (value :type Float%20%28single-precision%29))
  ;[1 1 1] Tests if this objective has been completed, and if so, records that and calls test for objectives completion from the objective manager
  (if (Utilities|IsValid (Variables|Default|GetobjectiveEntry))
    (Default|Update (Variables|Default|GetobjectiveEntry) value))
  (bind _output_get (Variables|Default|SettaskCompletionValue value))
  (bind _output_get_2 (Variables|Default|Setcomplete (>= _output_get (Variables|Default|GettaskCompletionTargetValue))))
  (if (and _output_get_2 (Utilities|IsValid (Variables|Default|GetobejectiveManager))) ; If the new value is at least the task completion target value, then inform the object manager that the objective is complete
    (Default|TestforObjectivesCompletion (Variables|Default|GetobejectiveManager))))

(fn ChangeCompletion
  (params (Increment :type Float%20%28single-precision%29))
  (CallFunction|SetCompletion (+ Increment (Variables|Default|GettaskCompletionValue))))

(fn Setup
  (params (objectiveManager :type Objective%20Manager%20Object%20Reference) (objectivePanel :type Objectives%20Panel%20Object%20Reference))
  ;[1 1 1] Sets up the objective and then calls setup for the Objective's Entry
  (Variables|Default|SetobejectiveManager objectiveManager)
  (bind _objective_entry (Default|AddObjectiveEntry objectivePanel))
  (bind _output_get (Variables|Default|SetobjectiveEntry _objective_entry))
  (Default|Setup _output_get (Variables|Default|GettaskName) (Variables|Default|GettaskCompletionTargetValue)))