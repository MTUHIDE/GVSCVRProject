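; BuildingMaster_BP is the RTS building master Blueprint, providing a configurable mesh, entrance, collision and a building HUD.
; Its construction script applies the display mesh, then sets up entrance and collision from that mesh.
; On BeginPlay it binds to the CameraPawnController's HUD request and creates the Building_HUD widget.
; DisplayHUD adds that widget to the viewport unconditionally, as its actor-equals-self check is left unwired.
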(event Custom|DisplayHUD
  (params (Actor :type Actor%20Object%20Reference))
  (if true
    (UserInterface|Viewport|AddtoViewport (Variables|Default|GetBuilding_HUD) 0)))

(event EventBeginPlay
  (bind _ascamera_pawn_controller (Utilities|Casting|CastToCameraPawnController (Game|GetPlayerController 0)))
  (bind _output_get (Variables|Refrences|SetControllerRef _ascamera_pawn_controller))
  (EventDispatchers|BindEventtoHUDRequest _output_get (EventDispatchers|CreateEvent :!event Custom|DisplayHUD))
  (bind _returnvalue (UserInterface|CreateWidget "/Game/RTS/HUDs/Building_HUD.Building_HUD_C"))
  (Variables|Default|SetBuilding_HUD _returnvalue))

(fn ConstructionScript
  (Components|StaticMesh|SetStaticMesh (Variables|Default|GetStaticMesh) (Variables|Default|GetDisplayMesh))
  (CallFunction|SetBuildingEntrance (Variables|Default|GetEntrance) (Variables|Default|GetStaticMesh))
  (CallFunction|SetBuildingCollision (Variables|Default|GetCollision) (Variables|Default|GetStaticMesh)))