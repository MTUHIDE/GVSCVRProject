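; Enemy base building for the RTS game that spawns enemy units.
; SpawnUnit creates an Enemy_NPC at the SpawnInPoint location and rotation, adjusting for collisions but always spawning, then gives it its default AI controller and returns it.
; SetCalendar and SetClock are stubs that only return false, and the construction script just calls the parent.
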(event Collision|EventActorBeginOverlap
  (params (OtherActor :type Actor%20Object%20Reference))
  (|CallParentFunction OtherActor) ; This node is disabled and will not be called.\nDrag off pins to build functionality.
)

(fn ConstructionScript
  (|CallParentFunction))

(fn SetCalendar
  (params (Date :type Array%20of%20Integers))
  (return false))

(fn SetClock
  (params (Time :type Array%20of%20Integers))
  (return false))

(fn SpawnUnit
  (bind _spawninpoint (Variables|Default|GetSpawnInPoint))
  (bind _returnvalue (Game|SpawnActorfromClass "/Game/RTS/Blueprints/AI/Enemies/Enemy_NPC.Enemy_NPC_C" (Math|Transform|MakeTransform (Transformation|GetWorldLocation _spawninpoint) (Transformation|GetWorldRotation _spawninpoint)) "AdjustIfPossibleButAlwaysSpawn" 0 0))
  ;[1 1 1] Spawns in the AI controller for this Pawn
  (Pawn|SpawnDefaultController _returnvalue)
  (return _returnvalue))