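; Base RTS NPC that randomizes its sex, body color and name, and exposes a busy state to its AI.
; The construction script tints a dynamic mesh material by a male-weighted random sex and stores name and sex in a profile.
; Names come from random enum entries, though GetRandomName's constant true condition always selects the male list.
; BeginPlay caches the NPC AI controller, whose Blackboard SetIsBusy updates.
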(event EventBeginPlay
  (Variables|Default|SetNPC_ControllerRef (.AsNPC%20AIController (Utilities|Casting|CastToNPC_AIController (AI|GetAIController self)))))

(event Collision|EventActorBeginOverlap
  (params (OtherActor :type Actor%20Object%20Reference)))

(event EventTick
  (params (DeltaSeconds :type Float%20%28single-precision%29)))

(fn ConstructionScript
  (CallFunction|RandomNPCFeatures))

(fn RandomNPCFeatures
  (bind _returnvalue (Rendering|Material|CreateDynamicMaterialInstance (Variables|Character|GetMesh) 0 0 "None" :!class /Script/Engine.PrimitiveComponent))
  (LocalVariables|SetMaterial_Instance _returnvalue)
  (if (<= (Math|Random|RandomIntegerinRange 0 2) 1)
    (Rendering|Material|SetVectorParameterValue (LocalVariables|GetMaterial_Instance) "BodyColor" (LocalVariables|GetMaleColor) :!class /Script/Engine.MaterialInstanceDynamic)
    (bind _name (CallFunction|GetRandomName "NewEnumerator0"))
    (Variables|Default|SetMyProfile (Utilities|Struct|MakeNPCProfile_Struct _name "NewEnumerator0"))
    (else
      (Rendering|Material|SetVectorParameterValue (LocalVariables|GetMaterial_Instance) "BodyColor" (LocalVariables|GetFemaleColor) :!class /Script/Engine.MaterialInstanceDynamic)
      (bind _name_2 (CallFunction|GetRandomName "NewEnumerator1"))
      (Variables|Default|SetMyProfile (Utilities|Struct|MakeNPCProfile_Struct _name_2 "NewEnumerator1")))))

(fn GetRandomName
  (params (Sex :type NPCSexType_ENUM%20Enum :default "NewEnumerator0"))
  (if true
    (return (Utilities|String|EnumtoString (Utilities|Enum|LiteralenumNPCName_Male_ENUM (Utilities|Enum|ByteToEnumNPCName_Male_ENUM (Math|Conversions|ToByte(Integer) (Math|Random|RandomIntegerinRange 0 (- (|GetNumEnumEntries) 1)))))))
    (else
      (return (Utilities|String|EnumtoString (Utilities|Enum|LiteralenumNPCName_Female_ENUM (Utilities|Enum|ByteToEnumNPCName_Female_ENUM (Math|Conversions|ToByte(Integer) (Math|Random|RandomIntegerinRange 0 (- (|GetNumEnumEntries) 1))))))))))

(fn SetIsBusy
  (params (IsBusy :type Boolean))
  (AI|Components|Blackboard|SetValueasBool (AI|GetBlackboard (Variables|Default|GetNPC_ControllerRef)) (Variables|Default|GetIsBusy) IsBusy)
  (return))