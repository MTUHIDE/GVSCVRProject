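; NPC_AIController is the AI controller for basic NPC pawns in the RTS game.
; On begin play it caches the player's CameraPawnController, initializes the NPC blackboard and runs the NPC behavior tree.
; On possess it stores the pawn as NPC_Basic.
; A custom NPCMovetoLocation event issues simple navigation moves to a given target location.
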(event EventBeginPlay
  (Variables|Default|SetCameraControllerReference (.AsCamera%20Pawn%20Controller (Utilities|Casting|CastToCameraPawnController (Game|GetPlayerController 0))))
  (Class|AIController|UseBlackboard "/Game/RTS/Blueprints/AI/NPC_Blackboard.NPC_Blackboard")
  (AI|RunBehaviorTree "/Game/RTS/Blueprints/AI/NPC_Behavior.NPC_Behavior"))

(event EventPossess
  (params (PossessedPawn :type Pawn%20Object%20Reference))
  (Variables|Default|SetPawnReference (.AsNPC%20Basic (Utilities|Casting|CastToNPC_Basic PossessedPawn))))

(event EventNPCMovetoLocation
  (params (TargetLocation :type Vector :default "0, 0, 0"))
  (AI|Navigation|SimpleMovetoLocation self TargetLocation))

(fn ConstructionScript)