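; A temporary debug actor that drives an RTS NPC by writing directly into its AI blackboard.
; Every tick it gets the NPC_AIController of ObjectToControl and pushes its own location as the destination vector, plus a task enum and, when valid, a destination object.
; An ApplyAtLocation flag acts as a one-shot trigger that writes the AtLocation bool and then resets itself.
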(event EventTick
  (params (DeltaSeconds :type Float%20%28single-precision%29))
  (bind _destination (Variables|Default|GetDestination))
  (bind _asnpc_aicontroller (Utilities|Casting|CastToNPC_AIController (AI|GetAIController (Variables|Default|GetObjectToControl))))
  (Utilities|FlowControl|Sequence
    (:then_0
      (if (Variables|Default|GetApplyAtLocation)
        (AI|Components|Blackboard|SetValueasBool (AI|GetBlackboard _asnpc_aicontroller) (Variables|Default|GetAtLocationName) (Variables|Default|GetAtLocation))
        (Variables|Default|SetApplyAtLocation false)))
    (:then_1
      (AI|Components|Blackboard|SetValueasVector (AI|GetBlackboard _asnpc_aicontroller) (Variables|Default|GetDestinationVectorName) (Transformation|GetActorLocation)))
    (:then_2
      (if (Utilities|IsValid _destination)
        (AI|Components|Blackboard|SetValueasObject (AI|GetBlackboard _asnpc_aicontroller) (Variables|Default|GetDestinationName) _destination)))
    (:then_3
      (AI|Components|Blackboard|SetValueasEnum (AI|GetBlackboard _asnpc_aicontroller) (Variables|Default|GetTaskAtDestinationName) (Variables|Default|GetTaskAtDestination)))))

(fn ConstructionScript)