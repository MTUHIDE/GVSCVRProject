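; Health component for RTS units that tracks hit points and destroys its owning actor when they run out.
; DealDamage subtracts damage from Health, and Tick watches for a negative value.
; A gate opened after being entered delays destruction by one tick, which helps resolve ties between units.
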(event EventBeginPlay)

(event EventTick
  (params (DeltaSeconds :type Float%20%28single-precision%29))
  (if (< (Variables|Default|GetHealth) 0.0)
    ;[1 1 1] kills it on the NEXT tick (helps with ties)
    (Utilities|FlowControl|Sequence
      (:then_0
        (Utilities|FlowControl|Gate true :!label _label
          (:Exit
            (Actor|DestroyActor (Components|GetOwner)))))
      (:then_1
        (goto _label Open)))))

(fn DealDamage
  (params (damage :type Float%20%28single-precision%29))
  (Variables|Default|SetHealth (- (Variables|Default|GetHealth) damage)))