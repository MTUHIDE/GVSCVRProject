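; RTS player controller with VR support that drives the camera pawn, unit commands and building placement.
; BeginPlay spawns the construction manager, ghost building and HUD; axis input, screen-edge scrolling and spring-arm zoom move the camera.
; Gamepad right trigger queues ghost construction or selects under the cursor, opening a gate that lets right-click move selected NPCs.
; With an HMD active, Tick copies headset rotation, yaw-offset, onto the controller's own transform.
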(event EventBeginPlay
  (bind _returnvalue (Math|Transform|MakeTransform "0, 0, 0"))
  ;[1 1 1] Begin Play
  (Utilities|FlowControl|Sequence
    (:then_0
      (Utilities|ReferenceCasts))
    (:then_1
      (bind _returnvalue_2 (Game|SpawnActorfromClass "/Game/RTS/Blueprints/Construction/ConstructionManager_BP.ConstructionManager_BP_C" _returnvalue "AlwaysSpawn" 0 0))
      (Variables|Default|SetConstructionManagerRef _returnvalue_2))
    (:then_2
      (bind _returnvalue_3 (Game|SpawnActorfromClass "/Game/RTS/Blueprints/Buildings/GhostBuilding_BP.GhostBuilding_BP_C" _returnvalue "AlwaysSpawn" 0 self 0))
      (Variables|Default|SetGhostBuildingRef _returnvalue_3))
    (:then_3
      (Input|SetInputModeGameandUI self 0 "LockInFullscreen" true)
      (Utilities|CreateHuds)
      (UserInterface|Viewport|AddtoViewport (Variables|References|GetMainHudRef_0) 0))))

(event EventTick
  (params (DeltaSeconds :type Float%20%28single-precision%29))
  (Utilities|FlowControl|Sequence
    (:then_0
      ;[1 1 1] Follow Cursor during Build Mode
      (if (Variables|Default|GetBuildModeActive)
        _))
    (:then_1
      (if (Class|HeadMountedDisplayFunctionLibrary|IsHeadMountedDisplayEnabled)
        (if (Class|HeadMountedDisplayFunctionLibrary|IsHeadMountedDisplayConnected)
          (Transformation|SetActorTransform self (CallFunction|VRRotationTransform)))))))

(event Input|ActionEvents|InputActionZoomIn
  (params (Key :type Key%20Structure :default "None"))
  (bind _camerapawnref (Variables|Default|GetCameraPawnRef))
  (bind _springarm (Variables|/Game/RTS/Blueprints/CameraPawn.CameraPawn_C|GetSpringArm _camerapawnref))
  ;[1 1 1] Zoom In and Out
  (:Pressed
    (Variables|/Script/Engine.SpringArmComponent|SetTargetArmLength _springarm (Math|Float|Clamp(Float) (- (Variables|/Script/Engine.SpringArmComponent|GetTargetArmLength _springarm) (Variables|Default|GetZoomSensitivity)) 5e+02 (Variables|Default|GetMaxArmDistance)))))

(event Input|ActionEvents|InputActionZoomOut
  (params (Key :type Key%20Structure :default "None"))
  (bind _camerapawnref (Variables|Default|GetCameraPawnRef))
  (bind _springarm (Variables|/Game/RTS/Blueprints/CameraPawn.CameraPawn_C|GetSpringArm _camerapawnref))
  ;[1 1 1] Zoom In and Out
  (:Pressed
    (Variables|/Script/Engine.SpringArmComponent|SetTargetArmLength _springarm (Math|Float|Clamp(Float) (+ (Variables|Default|GetZoomSensitivity) (Variables|/Script/Engine.SpringArmComponent|GetTargetArmLength _springarm)) 5e+02 (Variables|Default|GetMaxArmDistance)))))

(event Input|ActionEvents|InputActionZoomReset
  (params (Key :type Key%20Structure :default "None"))
  ;[1 1 1] Zoom Reset
  (:Pressed
    (Variables|/Script/Engine.SpringArmComponent|SetTargetArmLength (Variables|/Game/RTS/Blueprints/CameraPawn.CameraPawn_C|GetSpringArm (Variables|Default|GetCameraPawnRef)) 1.5e+03)))

(event Input|ActionEvents|InputActionDeselect
  (params (Key :type Key%20Structure :default "None"))
  (:Pressed
    (if (Variables|Default|GetBuildModeActive)
      (Default|KillGhost (Variables|Default|GetGhostBuildingRef))
      (Variables|Default|SetBuildModeActive false))))

(event Input|AxisEvents|InputAxisMoveRight
  (params (AxisValue :type Float%20%28single-precision%29))
  (bind _movementsensitivity (CallFunction|MovementSpeedCalculation))
  (bind _fastmovemultiplier (Variables|Default|GetFastMoveMultiplier))
  (bind _camerapawnref (Variables|Default|GetCameraPawnRef))
  (bind _transform (Utilities|MovementY AxisValue _movementsensitivity _fastmovemultiplier _camerapawnref))
  (bind (_location _rotation _scale) (Math|Transform|BreakTransform _transform))
  (bind (_x _y) (Math|Vector|BreakVector _location))
  ;[1 1 1] Movement Y
  (if (not (Variables|Default|GetDisableCamNav))
    (Transformation|SetActorTransform (Variables|Default|GetCameraPawnRef) (Math|Transform|MakeTransform (Math|Vector|MakeVector _x _y 1e+02) _rotation _scale))))

(event Input|AxisEvents|InputAxisMoveLeft
  (params (AxisValue :type Float%20%28single-precision%29))
  (bind _movementsensitivity (CallFunction|MovementSpeedCalculation))
  (bind _returnvalue (* -1 AxisValue))
  (bind _fastmovemultiplier (Variables|Default|GetFastMoveMultiplier))
  (bind _camerapawnref (Variables|Default|GetCameraPawnRef))
  (bind _transform (Utilities|MovementY _returnvalue _movementsensitivity _fastmovemultiplier _camerapawnref))
  (bind (_location _rotation _scale) (Math|Transform|BreakTransform _transform))
  (bind (_x _y) (Math|Vector|BreakVector _location))
  ;[1 1 1] Movement Y
  (if (not (Variables|Default|GetDisableCamNav))
    (Transformation|SetActorTransform (Variables|Default|GetCameraPawnRef) (Math|Transform|MakeTransform (Math|Vector|MakeVector _x _y 1e+02) _rotation _scale))))

(event Input|AxisEvents|InputAxisMoveForward
  (params (AxisValue :type Float%20%28single-precision%29))
  ;[1 1 1] Movement X
  (if (not (Variables|Default|GetDisableCamNav))
    (Transformation|SetActorTransform (Variables|Default|GetCameraPawnRef) (Utilities|MovementX (CallFunction|MovementSpeedCalculation) (Variables|Default|GetFastMoveMultiplier) AxisValue (Variables|Default|GetCameraPawnRef)))))

(event Input|AxisEvents|InputAxisMoveBackward
  (params (AxisValue :type Float%20%28single-precision%29))
  ;[1 1 1] Movement X
  (if (not (Variables|Default|GetDisableCamNav))
    (Transformation|SetActorTransform (Variables|Default|GetCameraPawnRef) (Utilities|MovementX (CallFunction|MovementSpeedCalculation) (Variables|Default|GetFastMoveMultiplier) (* -1 AxisValue) (Variables|Default|GetCameraPawnRef)))))

(event Input|MouseEvents|MouseX
  (params (AxisValue :type Float%20%28single-precision%29))
  ;[1 1 1] ScreenEdge Movement
  (if (not (Variables|Default|GetDisableCamNav))
    (bind (_deltaxspeed _deltayspeed) (Utilities|ScreenEdgeMovement))
    (Transformation|AddActorLocalOffset (Variables|Default|GetCameraPawnRef) (Math|Vector|MakeVector _deltaxspeed _deltayspeed 0.0) true false)))

(event Input|MouseEvents|MouseY
  (params (AxisValue :type Float%20%28single-precision%29))
  ;[1 1 1] ScreenEdge Movement
  (if (not (Variables|Default|GetDisableCamNav))
    (Utilities|ScreenEdgeMovement) ; enters at MouseY
  ))

(event Input|MouseEvents|RightMouseButton
  (params (Key :type Key%20Structure :default "None"))
  ;[1 1 1] Left Mouse Button
  (:Pressed
    (Utilities|FlowControl|Gate true
      (:Exit
        (Default|NPCMovetoLocation (stale Input|GamepadEvents|GamepadRightTrigger _asnpc_basic) (.Location (Collision|BreakHitResult (.HitResult (Class|PlayerController|GetHitResultUnderCursorforObjects (Variables|Default|GetSelectableObjectsENUM) true)))))))))

(event Input|GamepadEvents|GamepadRightTrigger
  (params (Key :type Key%20Structure :default "None"))
  (bind _selectableobjectsenum (Variables|Default|GetSelectableObjectsENUM))
  (bind _hitresult (Class|PlayerController|GetHitResultUnderCursorforObjects _selectableobjectsenum true))
  (bind (_bblockinghit _binitialoverlap _time _distance _location _impactpoint _normal _impactnormal _physmat _hitactor) (Collision|BreakHitResult _hitresult))
  ;[1 1 1] Left Mouse Button
  (:Pressed
    (if (Variables|Default|GetBuildModeActive)
      (if (|VerifyAsPlaceable)
        (bind _constructionstruct (Default|GetConstructionStruct (Variables|Default|GetGhostBuildingRef)))
        (Default|QueueConstruction (Variables|Default|GetConstructionManagerRef) _constructionstruct)
        (Default|KillGhost (Variables|Default|GetGhostBuildingRef)))
      (elif (!= _hitactor 0)
        (bind _asnpc_basic (Utilities|Casting|CastToNPC_Basic _hitactor)
          (:then
            (Utilities|FlowControl|Gate true) ; enters at Open
          )
          (:CastFailed
            (Default|CallHUDRequest0 _hitactor)
            (Utilities|FlowControl|Gate true) ; enters at Close
          ))))))

(fn ConstructionScript)

(fn VRRotationTransform
  (bind _devicerotation (Class|HeadMountedDisplayFunctionLibrary|GetOrientationandPosition))
  (bind _self self)
  (bind _returnvalue (Transformation|GetActorTransform _self))
  (return (Math|Transform|MakeTransform (.location _returnvalue) (Math|Rotator|MakeRotator (.roll _devicerotation) (.pitch _devicerotation) (- (.yaw _devicerotation) 7e+01)) (.scale _returnvalue))))