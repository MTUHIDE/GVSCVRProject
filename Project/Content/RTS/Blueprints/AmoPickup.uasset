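; AmoPickup is an ammo pickup that adds AmoAmount to a TopDownCharacter's Amo when that character overlaps its Sphere component.
; The overlap event reads the character's Amo and MaxAmo, and applies the pickup and destroys the actor only if the whole amount fits.
; Full or would-overflow cases do nothing, as the nodes that set Amo to MaxAmo and destroy the pickup are unconnected.
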(event OnComponentBeginOverlap(Sphere)
  (params (OverlappedComponent :type Primitive%20Component%20Object%20Reference) (OtherActor :type Actor%20Object%20Reference) (OtherComp :type Primitive%20Component%20Object%20Reference) (OtherBodyIndex :type Integer) (bFromSweep :type Boolean) (SweepResult :type Hit%20Result%20Structure%20%28by%20ref%29))
  (bind _astop_down_character (Utilities|Casting|CastToTopDownCharacter OtherActor))
  (Variables|Default|SetAmo (Variables|/Game/RTS/Blueprints/TopDownCharacter.TopDownCharacter_C|GetAmo _astop_down_character))
  (Variables|Default|SetMaxAmo (Variables|/Game/RTS/Blueprints/TopDownCharacter.TopDownCharacter_C|GetMax%20Amo _astop_down_character))
  (Variables|Default|SetAmoPlusAmoAmount (+ (Variables|/Game/RTS/Blueprints/TopDownCharacter.TopDownCharacter_C|GetAmo _astop_down_character) (Variables|Default|GetAmoAmount))) ; Variables have been initialized
  (if (not (>= (Variables|Default|GetAmo) (Variables|Default|GetMaxAmo))) ; If Amo is already filled do nothing
    (if (not (> (Variables|Default|GetAmoPlusAmoAmount) (Variables|Default|GetMaxAmo))) ; If Amo + AmoAmount overfills
      (if (<= (Variables|Default|GetAmoPlusAmoAmount) (Variables|Default|GetMaxAmo)) ; If there is room for all of the new Amo
        (Variables|/Game/RTS/Blueprints/TopDownCharacter.TopDownCharacter_C|SetAmo _astop_down_character (Variables|Default|GetAmoPlusAmoAmount))
        (Actor|DestroyActor)))))

(event EventBeginPlay)

(event Collision|EventActorBeginOverlap
  (params (OtherActor :type Actor%20Object%20Reference)))

(event EventTick
  (params (DeltaSeconds :type Float%20%28single-precision%29)))

(fn ConstructionScript)